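; First-person player character for a story-driven ghost game, handling movement, interaction, object inspection, zoom and menus.
; Box overlaps and a camera box trace find interface-based objects; inspecting locks movement and turns the attach point.
; Looking back freezes cached movement vectors, so walking keeps its heading.
; It also scripts the timeline-driven wake-up intro, plays data-table or direct dialogue with audio, and arms tagged ghosts after two inspections.
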(event OnComponentBeginOverlap(Box)
  (params (OverlappedComponent :type Primitive%20Component%20Object%20Reference) (OtherActor :type Actor%20Object%20Reference) (OtherComp :type Primitive%20Component%20Object%20Reference) (OtherBodyIndex :type Integer) (bFromSweep :type Boolean) (SweepResult :type Hit%20Result%20Structure%20%28by%20ref%29))
  (bind _returnvalue (Utilities|DoesObjectImplementInterface OtherActor "/Game/Blueprints/Interfaces/InteractiveObj_BPI.InteractiveObj_BPI_C"))
  ;[1 1 1] Object Detection
  (Variables|Default|SetInteractiveObj _returnvalue)
  (if _returnvalue
    (Variables|Default|SetTargetActor OtherActor)
    (Class|InteractiveObjBPI|Detected(Message) (Variables|Default|GetTargetActor))
    (else
      (Variables|Default|SetTargetActor 0))))

(event OnComponentEndOverlap(Box)
  (params (OverlappedComponent :type Primitive%20Component%20Object%20Reference) (OtherActor :type Actor%20Object%20Reference) (OtherComp :type Primitive%20Component%20Object%20Reference) (OtherBodyIndex :type Integer))
  ;[1 1 1] Object Detection
  (Variables|Default|SetInteractiveObj false)
  (Class|InteractiveObjBPI|OutOfRange(Message) OtherActor))

(event Custom|StoreVariablesTick
  (Utilities|FlowControl|Sequence
    (:then_0
      (|SoreDirectionalVectors))))

(event Custom|DOF
  (bind _camera (Variables|Default|GetCamera))
  ;[1 1 1] DOF
  (if (Variables|Default|GetbActorInspect)
    (Variables|/Script/Engine.CameraComponent|SetPostProcessSettings _camera (Utilities|Struct|MakePostProcessSettings 1.0 1.5e+02 1e+02))
    (else
      (Variables|/Script/Engine.CameraComponent|SetPostProcessSettings _camera (Utilities|Struct|MakePostProcessSettings 4.0)))))

(event Custom|WakeUpEffect
  ;[1 1 1] WakeUpEffect
  (Variables|Default|SetGameStarted true)
  (if (Variables|Default|GetPlayStartAnimation)
    (Transformation|SetWorldTransform (Variables|Default|GetCamera) (Transformation|GetWorldTransform (Variables|Default|GetCameraLerpStart)) false false)
    (CameraFades|StartCameraFade :self (Game|GetPlayerCameraManager 0) :FromAlpha 1.0 :Duration 2.0)
    (Utilities|FlowControl|Delay 2.0)
    (CameraFades|StartCameraFade :self (Game|GetPlayerCameraManager 0) :ToAlpha 1.0 :Duration 2.0 :bHoldWhenFinished true)
    (Utilities|FlowControl|Delay 2.0)
    (CameraFades|StartCameraFade :self (Game|GetPlayerCameraManager 0) :FromAlpha 1.0 :Duration 2.0 :bHoldWhenFinished true)
    (bind _newtrack_0 (Timeline|LerpCamera PlayFromStart)
      (:Update
        (Transformation|SetWorldTransform (Variables|Default|GetCamera) (Math|Transform|Lerp(Transform) (Transformation|GetWorldTransform (Variables|Default|GetCameraLerpStart)) (Transformation|GetWorldTransform (Variables|Default|GetCameraLerpEnd)) _newtrack_0) false false))
      (:Finished
        (CallFunction|UpdateTextandPlayAudio 6 "Thirsty dialogue 1" false)
        (CallFunction|LerpActorLocation 1)))
    (else
      (Variables|Default|SetWakeUpCompleted true))))

(event Custom|LerpLocationOfPlayer
  (params (InitialPos :type Actor%20Object%20Reference) (FinalPos :type Actor%20Object%20Reference))
  (bind _outactors (Actor|GetAllActorswithTag "InitialPos1"))
  (bind _outactors_2 (Actor|GetAllActorswithTag "FinalPos1"))
  (bind _newtrack_0 (Timeline|LerpLocation PlayFromStart)
    (:Update
      (Transformation|SetWorldLocation (Variables|Collision|GetCapsuleComponent) (Math|Vector|Lerp(Vector) (Transformation|GetWorldLocation (Variables|Collision|GetCapsuleComponent)) (Transformation|GetActorLocation (Utilities|Array|Get(acopy) _outactors_2)) _newtrack_0) false false)
      (Transformation|SetWorldRotation (Variables|Collision|GetCapsuleComponent) (Math|Rotator|Lerp(Rotator) (Transformation|GetActorRotation (Utilities|Array|Get(acopy) _outactors)) (Transformation|GetActorRotation (Utilities|Array|Get(acopy) _outactors_2)) _newtrack_0) false false))))

(event Custom|LerpActorLocation
  (params (lerpactorindex :type Integer))
  (Variables|Default|SetInitialActorRot (Transformation|GetActorRotation))
  (Variables|Default|SetInitialActorLerpLoc (Transformation|GetActorLocation))
  (bind _outactors (Actor|GetAllActorswithTag (Utilities|String|StringToName (Utilities|String|Append (Utilities|String|ToString(Name) (Variables|Default|Getlerpnametag)) (Utilities|String|ToString(Integer) lerpactorindex)))))
  (bind _newtrack_0 (Timeline|lerpactor PlayFromStart)
    (:Update
      (Transformation|SetActorLocation (Math|Vector|Lerp(Vector) (Variables|Default|GetInitialActorLerpLoc) (Transformation|GetActorLocation (Utilities|Array|Get(acopy) _outactors)) _newtrack_0) false false))
    (:Finished
      (CallFunction|LerpFinished lerpactorindex))))

(event Custom|LerpFinished
  (params (lerpindex :type Integer))
  (if (== lerpindex 1)
    (Utilities|FlowControl|DoOnce false
      (:Completed
        (CallFunction|LerpActorLocation 2)
        (Utilities|FlowControl|Delay 4.0)
        ;[1 1 1] CloseDoor
        (Variables|Default|SetWakeUpCompleted true)
        (bind _outactors (Actor|GetAllActorswithTag "nikkiroomdoor"))
        (bind _asdoor_bp (Utilities|Casting|CastToDoor_BP (Utilities|Array|Get(acopy) _outactors)))
        (Default|OpenDoor _asdoor_bp)
        (CallFunction|UpdateTextandPlayAudio 7 "Thirsty Dialogue 2" false)))))

(event Custom|AddToNumberOfInspections
  (bind _output_get (Variables|Default|SetTopFloorInspections (+ (Variables|Default|GetTopFloorInspections) 1)))
  (if (>= _output_get 2)
    (bind _outactors (Actor|GetAllActorswithTag "ghost1"))
    (bind _asghost_bp (Utilities|Casting|CastToGhost_BP (Utilities|Array|Get(acopy) _outactors)))
    (Variables|/Game/Blueprints/Actors/NPC/Ghost_BP.Ghost_BP_C|SetActivateTrigger _asghost_bp true)
    (CallFunction|MakeItRain)
    (else
      (Development|PrintString "Not2"))))

(event Custom|MakeItRain
  (Utilities|FlowControl|Delay 3.0)
  (CallFunction|UpdateTextandPlayAudio 0 "The weather doesn't look good. I should head back!" false "/Game/Assets/Audio/TestVoiceOvers/4.4")
  (bind _outactors (Actor|GetAllActorswithTag "ghost2"))
  (bind _asghost_bp (Utilities|Casting|CastToGhost_BP (Utilities|Array|Get(acopy) _outactors)))
  (Variables|/Game/Blueprints/Actors/NPC/Ghost_BP.Ghost_BP_C|SetActivateTrigger _asghost_bp true))

(event Custom|LookPitch
  ;[0 0 0] Locomotion
  ;;[1 1 1] Look
  (if (Variables|Default|GetbLookingBack)
    (Pawn|Input|AddControllerPitchInput (/ (Input|AxisValues|GetLookup) 1e+01))
    (else
      (Pawn|Input|AddControllerPitchInput (Input|AxisValues|GetLookup)))))

(event Custom|LookYaw
  ;[0 0 0] Locomotion
  ;;[1 1 1] Look
  (if (Variables|Default|GetbLookingBack)
    (Pawn|Input|AddControllerYawInput (/ (Input|AxisValues|GetTurn) 1e+01))
    (else
      (Pawn|Input|AddControllerYawInput (Input|AxisValues|GetTurn)))))

(event Custom|TurnObject
  ;[1 1 1] Inspect Point
  (Transformation|AddRelativeRotation (Variables|Default|GetAttachPoint) (Math|Rotator|MakeRotator (Input|AxisValues|GetLookup) 0.0 (* (Input|AxisValues|GetTurn) -1.0)) false false))

(event Custom|Inspect
  (bind _attachpoint (Variables|Default|GetAttachPoint))
  ;[1 1 1] Inspect
  (if (Variables|Default|GetbActorInspect)
    (Class|InteractiveObjBPI|KeepBack(Message) (Variables|Default|GetInspectActor) (Transformation|GetWorldLocation _attachpoint) (Transformation|GetWorldRotation _attachpoint))
    (Utilities|FlowControl|Delay 0.5)
    (Variables|Default|SetbActorInspect false)
    (Transformation|SetRelativeRotation (Variables|Default|GetAttachPoint) "0, 0, 0" false false)
    (else
      (CallFunction|ActorInteract))))

(event Custom|ActorInteract
  ;[1 1 1] Object Action
  (if (Variables|Default|GetInteractiveObj)
    (bind (_out_hit_blocking_hit _out_hit_time _out_hit_distance _out_hit_location _out_hit_normal _out_hit_hit_actor) (CallFunction|FindInteractiveActor (Variables|Default|GetTargetActor)))
    (if (and _out_hit_blocking_hit (Utilities|DoesObjectImplementInterface _out_hit_hit_actor "/Game/Blueprints/Interfaces/InteractiveObj_BPI.InteractiveObj_BPI_C"))
      (bind (_actorout _battached) (Class|InteractiveObjBPI|Interact(Message) _out_hit_hit_actor self))
      (bind _output_get (Variables|Default|SetInspectActor _actorout))
      (if (not (Actor|ActorHasTag _output_get "door"))
        (Variables|Default|SetbActorInspect _battached)))
    (else
      (Development|PrintString "Fail"))))

(event Custom|SetHead
  ;[1 1 1] SetResetHead
  (bind _looktime (Timeline|LookUp PlayFromStart)
    (:Update
      (if (> (.pitch (Pawn|GetControlRotation (Pawn|GetController) :!class /Script/Engine.Controller)) 1.5e+02)
        (CallFunction|ResetHead 0.0 (* _looktime 0.5))
        (else
          (CallFunction|ResetHead 0.0 (* _looktime -0.5)))))))

(event Custom|FindMenu
  (if (Variables|Default|GetbStartMenu)
    (bind _outactors (Actor|GetAllActorsOfClass "/Game/Blueprints/Pawns/MainMenu_BP.MainMenu_BP_C"))
    (Pawn|Possess (Pawn|GetController) (Utilities|Array|Get(acopy) _outactors))))

(event Custom|UpdateTextAndPlayAudio
  (params (RowNumber :type Integer) (TextToDisplay :type Text) (ChooseFromTable :type Boolean) (SoundWave :type Sound%20Wave%20Object%20Reference))
  (bind _audio (Variables|Default|GetAudio))
  (bind _audio_2 (Variables|Default|GetAudio))
  ;[1 1 1] Dialogue Audio and text
  (Widget|SetVisibility (Variables|Default|GetDialogueWidget) "Visible")
  (if ChooseFromTable
    (bind _outrownames (DataTable|GetDataTableRowNames "/Game/Widgets/DialogueData.DialogueData"))
    (bind _returnvalue (Utilities|GetDataTableRow "/Game/Widgets/DialogueData.DialogueData" (Utilities|Array|Get(acopy) _outrownames (- RowNumber 1)))
      (:then
        (Default|UpdateDialogue (Variables|Default|GetDialogueWidget) (.DialogueText (Utilities|Struct|BreakDialogueStruct _returnvalue)))
        (Audio|Components|Audio|SetSound _audio_2 (.AudioAsset (Utilities|Struct|BreakDialogueStruct _returnvalue)))
        (Audio|Components|Audio|Play _audio_2 0.0)
        (Development|PrintString (Utilities|String|ToString(Text) (.DialogueText (Utilities|Struct|BreakDialogueStruct _returnvalue)))))
      (:RowNotFound
        (Development|PrintString "RowNotFound")))
    (else
      (Default|UpdateDialogue (Variables|Default|GetDialogueWidget) TextToDisplay)
      (Audio|Components|Audio|SetSound _audio SoundWave)
      (Audio|Components|Audio|Play _audio 0.0)
      (Development|PrintString (Utilities|String|ToString(Text) TextToDisplay)))))

(event EventTick
  (params (DeltaSeconds :type Float%20%28single-precision%29))
  (CallFunction|StoreVariablesTick)
  (CallFunction|CheckAudioPlayState))

(event EventBeginPlay
  (CallFunction|AddMainMenu)
  (CallFunction|DialogueWidgetAdd))

(event Input|ActionEvents|InputActionInteract
  (params (Key :type Key%20Structure :default "None"))
  ;[1 1 1] Press E to Interact
  (:Pressed
    (CallFunction|Inspect)))

(event Input|ActionEvents|InputActionViewModifier
  (params (Key :type Key%20Structure :default "None"))
  ;[0 0 0] Locomotion
  ;;[1 1 1] LookBack
  (:Pressed
    (if (not (Variables|Default|GetbActorInspect))
      (Variables|Default|SetbLookingBack true)
      (if (Variables|Default|GetWakeUpCompleted)
        (Pawn|Input|AddControllerYawInput (+ (Input|AxisValues|GetTurn) 5e+02)))))
  (:Released
    (if (Variables|Default|GetbLookingBack)
      (if (not (Variables|Default|GetbActorInspect))
        (if (Variables|Default|GetWakeUpCompleted)
          (Pawn|Input|AddControllerYawInput (- (Input|AxisValues|GetTurn) 5e+02))
          (Variables|Default|SetbLookingBack false))))))

(event Input|ActionEvents|InputActionMagnify
  (params (Key :type Key%20Structure :default "None"))
  ;[1 1 1] Zoom
  (:Pressed
    (bind _fov (Timeline|SetFov Play)
      (:Update
        (Camera|SetFieldOfView (Variables|Default|GetCamera) _fov))))
  (:Released
    (Timeline|SetFov Reverse)))

(event Input|ActionEvents|InputActionPause
  (params (Key :type Key%20Structure :default "None"))
  (:Pressed
    (CallFunction|AddMainMenu)))

(event Input|AxisEvents|InputAxisForward
  (params (AxisValue :type Float%20%28single-precision%29))
  ;[0 0 0] Locomotion
  ;;[1 1 1] Movement
  (if (not (Variables|Default|GetbActorInspect))
    (if (Variables|Default|GetWakeUpCompleted)
      (Pawn|Input|AddMovementInput (* (Variables|Default|GetForwardVector) AxisValue) 1.0 false))))

(event Input|AxisEvents|InputAxisStrafe
  (params (AxisValue :type Float%20%28single-precision%29))
  ;[0 0 0] Locomotion
  ;;[1 1 1] Movement
  (if (not (Variables|Default|GetbActorInspect))
    (if (Variables|Default|GetWakeUpCompleted)
      (Pawn|Input|AddMovementInput (* (Variables|Default|GetRightVector) AxisValue) 1.0 false))))

(event Input|AxisEvents|InputAxisTurn
  (params (AxisValue :type Float%20%28single-precision%29))
  ;[1 1 1] Executes
  (if (Variables|Default|GetbActorInspect)
    (CallFunction|TurnObject)
    (elif (Variables|Default|GetWakeUpCompleted)
      (CallFunction|LookYaw))))

(event Input|AxisEvents|InputAxisLookup
  (params (AxisValue :type Float%20%28single-precision%29))
  ;[1 1 1] Executes
  (if (not (Variables|Default|GetbActorInspect))
    (if (Variables|Default|GetWakeUpCompleted)
      (CallFunction|LookPitch))))

(event Input|KeyboardEvents|Escape
  (params (Key :type Key%20Structure :default "None"))
  (:Pressed
    (CallFunction|AddMainMenu)))

(fn ConstructionScript)

(fn FindInteractiveActor
  (params (Target :type Actor%20Object%20Reference))
  (bind _camera (Variables|Default|GetCamera))
  (bind _outhit (Class|KismetSystemLibrary|BoxTraceSingleforObjects (Transformation|GetWorldLocation (Variables|Default|GetCamera)) (+ (* (Math|Vector|GetForwardVector (Variables|Default|GetCamera)) 2e+02) (Transformation|GetWorldLocation _camera)) "20.000000,20.000000,20.000000" (Transformation|GetWorldRotation _camera) (Utilities|Array|MakeArray "ObjectTypeQuery1" "ObjectTypeQuery2") false (Utilities|Array|MakeArray 0) "ForDuration" true))
  (return (.bblockinghit _outhit) (.time _outhit) (.distance _outhit) (.location _outhit) (.normal _outhit) (.hitactor _outhit) (.hitcomponent _outhit)))

(fn ResetHead
  (params (PitchAmount :type Float%20%28single-precision%29) (Time :type Float%20%28single-precision%29))
  (bind _returnvalue (Pawn|GetController))
  (bind _returnvalue_2 (Pawn|GetControlRotation _returnvalue :!class /Script/Engine.Controller))
  (Pawn|SetControlRotation _returnvalue (Math|Rotator|MakeRotator (.roll _returnvalue_2) (+ Time (.pitch _returnvalue_2)) (.yaw _returnvalue_2))))

(fn CheckAudioPlayState
  (Utilities|FlowControl|Sequence
    (:then_0
      (if (Math|Boolean|NotEqual(Boolean) (Variables|Default|GetAudioPlaying) (Audio|Components|Audio|IsPlaying (Variables|Default|GetAudio)))
        (if (Variables|Default|GetAudioPlaying)
          (Development|PrintString "Audio End")
          (Utilities|FlowControl|DoOnce false :!label _label
            (:Completed
              (Default|FadeoutEvent (Variables|Default|GetDialogueWidget))
              (goto _label_2 Reset)))
          (else
            (Development|PrintString "Audio Start")
            (Utilities|FlowControl|DoOnce false :!label _label_2
              (:Completed
                (Default|FadeinEvent (Variables|Default|GetDialogueWidget))
                (goto _label Reset)))))))
    (:then_1
      (Variables|Default|SetAudioPlaying (Audio|Components|Audio|IsPlaying (Variables|Default|GetAudio))))))

(fn AddMainMenu
  (Utilities|IsValid (Variables|Default|GetMainMenuWidget)
    (:Is%20Valid
      (UserInterface|Viewport|AddtoViewport (Variables|Default|GetMainMenuWidget) 0)
      (Game|SetGamePaused true))
    (:Is%20Not%20Valid
      (bind _returnvalue (UserInterface|CreateWidget "/Game/Widgets/MainMenu_Widget2.MainMenu_Widget2_C"))
      (bind _output_get (Variables|Default|SetMainMenuWidget _returnvalue))
      (UserInterface|Viewport|AddtoViewport _output_get 0))))

(fn DialogueWidgetAdd
  (bind _returnvalue (UserInterface|CreateWidget "/Game/Widgets/Dialogue_Widget.Dialogue_Widget_C"))
  (UserInterface|Viewport|AddtoViewport _returnvalue 0)
  (bind _output_get (Variables|Default|SetDialogueWidget _returnvalue))
  (Widget|SetVisibility _output_get "Hidden"))