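; Interactive pickup actor that a character lifts to an attach point for inspection, then returns to its original place.
; Interact spawns an inspection light actor; Tick then interpolates the mesh toward the attach point's location and rotation, with the light following its position.
; KeepBack plays a timeline returning the mesh to its starting transform, destroys the light when finished, and increments the ProgressTracker objective only once.
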(event Custom|InspectObject
  ;[1 1 1] Inspect Object
  (if (Variables|Default|GetbInspect)
    (|InterpolateLocation)
    (|InterpolateRotation)))

(event Custom|KeepObjectBack
  ;[1 1 1] Place Object Back
  (if (not (Variables|Default|GetbKeepingBack))
    (bind _time (Timeline|PlaceObject PlayFromStart)
      (:Update
        (Transformation|SetWorldLocationAndRotation (Variables|Character|GetMesh) (Math|Vector|Lerp(Vector) (Variables|Default|GetSnapLocation) (Variables|Default|GetInitialLocation) _time) (Math|Rotator|Lerp(Rotator) (Variables|Default|GetSnapRotation) (Variables|Default|GetInitialRotation) _time true) false true))
      (:Finished
        (CallFunction|ObjectKept)))))

(event Custom|SpawnLight
  (bind _attachpoint (Variables|Default|GetAttachPoint))
  ;[1 1 1] Spawn Light
  (bind _returnvalue (Game|SpawnActorfromClass "/Game/Blueprints/Actors/Attachments/InspectLights_BP.InspectLights_BP_C" (Math|Transform|MakeTransform (Transformation|GetWorldLocation _attachpoint) (Math|Rotator|MakeRotator 0.0 0.0 (+ (.yaw (Transformation|GetWorldRotation _attachpoint)) 1.8e+02)) "1,1,1") "Undefined" 0 0))
  (Variables|Default|SetLights _returnvalue))

(event Custom|ObjectKept
  (Variables|Default|SetbKeepingBack false)
  (Variables|Default|SetbInspect false)
  (Actor|DestroyActor (Variables|Default|GetLights)))

(event Custom|ObjectiveDone
  (if (not (Variables|Default|GetbObjectiveComplete))
    (bind _outactors (Actor|GetAllActorsOfClass "/Game/Blueprints/Actors/Helpers/ProgressTracker_BP.ProgressTracker_BP_C"))
    (Default|IncrementObjective (Utilities|Array|Get(acopy) _outactors) (Variables|Default|GetObjectiveLevel))
    (Variables|Default|SetbObjectiveComplete true)))

(event EventBeginPlay
  (bind _mesh (Variables|Character|GetMesh))
  (bind _mesh_2 (Variables|Character|GetMesh))
  (bind _returnvalue (Transformation|GetWorldRotation _mesh))
  (bind _returnvalue_2 (Transformation|GetWorldLocation _mesh_2))
  (|CallParentFunction)
  ;[1 1 1] Variable Init
  (Variables|Default|SetSnapLocation _returnvalue_2)
  (Variables|Default|SetInitialLocation _returnvalue_2)
  (Variables|Default|SetInitialRotation _returnvalue)
  (Variables|Default|SetSnapRotation _returnvalue))

(event EventTick
  (params (DeltaSeconds :type Float%20%28single-precision%29))
  (|CallParentFunction DeltaSeconds)
  (CallFunction|InspectObject))

(fn ConstructionScript
  (|CallParentFunction)
  (Components|StaticMesh|SetStaticMesh (Variables|Character|GetMesh) "/Game/Assets/Meshes/Environment/Props/remote.remote"))

(fn Interact
  (params (Actor :type Actor%20Object%20Reference))
  (bind _ascharacter_base_bp (Utilities|Casting|CastToCharacterBase_BP Actor))
  (Default|SetHead _ascharacter_base_bp)
  (Variables|Default|SetSnapLocation (Variables|Default|GetInitialLocation))
  (Variables|Default|SetSnapRotation (Variables|Default|GetInitialRotation))
  (Variables|Default|SetAttachPoint (Variables|/Game/Blueprints/Pawns/CharacterBase_BP.CharacterBase_BP_C|GetAttachPoint _ascharacter_base_bp))
  (if (not (Variables|Default|GetbKeepingBack))
    (Variables|Default|SetbInspect true)
    (CallFunction|SpawnLight)
    (return self true)))

(fn KeepBack
  (params (CurrentLocation :type Vector :default "0, 0, 0") (CurrentRotation :type Rotator :default "0, 0, 0"))
  (CallFunction|KeepObjectBack)
  (Variables|Default|SetbKeepingBack true)
  (CallFunction|ObjectiveDone)
  (return false))