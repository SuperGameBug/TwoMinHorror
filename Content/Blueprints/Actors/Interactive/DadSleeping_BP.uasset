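; Interactive sleeping-dad actor that has the player character comment, with subtitle and voice line, that he fell asleep watching the match.
; A box overlap with the player's base capsule toggles a HUD_UMG prompt and an in-range flag.
; Interact plays the line once, guarded by EffectDone, which also blocks later prompts.
; Disconnected leftovers hold a longer mom dialogue leading to the top-door opening event, plus a physics impulse.
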(event OnComponentBeginOverlap(Box)
  (params (OverlappedComponent :type Primitive%20Component%20Object%20Reference) (OtherActor :type Actor%20Object%20Reference) (OtherComp :type Primitive%20Component%20Object%20Reference) (OtherBodyIndex :type Integer) (bFromSweep :type Boolean) (SweepResult :type Hit%20Result%20Structure%20%28by%20ref%29))
  (Utilities|Casting|CastToCharacterBase_BP OtherActor)
  (if (and (not (Variables|Default|GetEffectDone)) (Components|ComponentHasTag OtherComp "BaseCapsule"))
    (Utilities|IsValid (Variables|Default|GetPressEWidget)
      (:Is%20Valid
        _)
      (:Is%20Not%20Valid
        (bind _returnvalue (UserInterface|CreateWidget "/Game/Blueprints/UMG/UserInterFace/HUD_UMG.HUD_UMG_C"))))
    (bind _output_get (Variables|Default|SetPressEWidget _returnvalue))
    (UserInterface|Viewport|AddtoViewport _output_get 0)
    (Variables|Default|SetPlayerInRange true)))

(event OnComponentEndOverlap(Box)
  (params (OverlappedComponent :type Primitive%20Component%20Object%20Reference) (OtherActor :type Actor%20Object%20Reference) (OtherComp :type Primitive%20Component%20Object%20Reference) (OtherBodyIndex :type Integer))
  (Utilities|Casting|CastToCharacterBase_BP OtherActor)
  (if (Components|ComponentHasTag OtherComp "BaseCapsule")
    (Widget|RemovefromParent (Variables|Default|GetPressEWidget))
    (Variables|Default|SetPlayerInRange false)))

(event Custom|SleepingDialogue)

(event Custom|WhosThere
  (params (Character :type Character%20Base%20BP%20Object%20Reference)))

(event Custom|OpenTopDoorAndEffect
  (bind _outactors (Actor|GetAllActorswithTag "topdoor"))
  (bind _asdoor_bp (Utilities|Casting|CastToDoor_BP (Utilities|Array|Get(acopy) _outactors)))
  (Default|OpenDoor _asdoor_bp)
  (Variables|/Game/Blueprints/Actors/Interactive/Door_BP.Door_BP_C|SetDisableControl _asdoor_bp false))

(event EventBeginPlay)

(fn ConstructionScript)

(fn Detected
  (return false))

(fn InfoBubbleDown
  (return false))

(fn InfoBubbleUp
  (return false))

(fn Interact
  (params (Actor :type Actor%20Object%20Reference))
  (bind _ascharacter_base_bp (Utilities|Casting|CastToCharacterBase_BP Actor)
    (:then
      (if (Variables|Default|GetEffectDone)
        _
        (else
          (Variables|Default|SetEffectDone true)
          (Default|UpdateTextandPlayAudio _ascharacter_base_bp 0 "Must have fallen asleep watching the match." false "/Game/Assets/Audio/VoiceOvers/Nikki/3-_Must_have_fallen_asleep_watching_the_match.3-_Must_have_fallen_asleep_watching_the_match"))))
    (:CastFailed
      _))
  (return 0 false))

(fn KeepBack
  (params (CurrentLocation :type Vector :default "0, 0, 0") (CurrentRotation :type Rotator :default "0, 0, 0"))
  (return false))

(fn OutOfRange
  (return false))