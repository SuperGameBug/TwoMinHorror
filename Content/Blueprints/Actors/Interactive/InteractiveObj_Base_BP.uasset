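; Base Blueprint for interactive objects that show billboard prompts as they are detected, go out of range or are interacted with.
; The construction script applies the configurable mesh, and the detection, range and info-bubble functions toggle pointer and interaction billboards, with Inspecting hiding the pointer when out of range.
; Interact removes the HUD, prints the passed actor's name and calls InteractUIMessage on the first ViewHUD found.
; KeepBack is a stub, and HUD creation is unwired.
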(event Custom|PromptInteraction
  (Rendering|SetVisibility (Variables|Default|GetInteractionBill) true false))

(event EventBeginPlay)

(event EventTick
  (params (DeltaSeconds :type Float%20%28single-precision%29)))

(fn ConstructionScript
  (Components|StaticMesh|SetStaticMesh (Variables|Default|GetMesh) (Variables|Default|GetMeshObject)))

(fn Detected
  (CallFunction|PromptInteraction)
  (Rendering|SetVisibility (Variables|Default|GetPointerBill) false false)
  (Rendering|SetVisibility (Variables|Default|GetInteractionBill) true false)
  (return false))

(fn InfoBubbleDown
  (Rendering|SetVisibility (Variables|Default|GetPointerBill) false false)
  (Rendering|SetVisibility (Variables|Default|GetInteractionBill) false false)
  (return false))

(fn InfoBubbleUp
  (Rendering|SetVisibility (Variables|Default|GetInteractionBill) false false)
  (Rendering|SetVisibility (Variables|Default|GetPointerBill) true false)
  (return false))

(fn Interact
  (params (Actor :type Actor%20Object%20Reference))
  (Widget|RemovefromParent (Variables|Default|GetHUD))
  (Development|PrintString (Utilities|GetDisplayName Actor))
  (bind _outactors (Actor|GetAllActorsOfClass "/Game/Blueprints/UMG/ViewHUD.ViewHUD_C"))
  (Class|UIBPI|InteractUI(Message) (Utilities|Array|Get(acopy) _outactors))
  (return 0 false))

(fn KeepBack
  (params (CurrentLocation :type Vector :default "0, 0, 0") (CurrentRotation :type Rotator :default "0, 0, 0"))
  (return false))

(fn OutOfRange
  (Rendering|SetVisibility (Variables|Default|GetInteractionBill) false false)
  (if (Variables|Default|GetbInspecting)
    (Rendering|SetVisibility (Variables|Default|GetPointerBill) false false)
    (else
      (Rendering|SetVisibility (Variables|Default|GetPointerBill) true false)))
  (return false))