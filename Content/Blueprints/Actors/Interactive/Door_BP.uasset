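; Interactive door actor that swings its mesh open or shut with a timeline, toggled by a FlipFlop, and can start open.
; Interact toggles it, or while control is disabled sends text and audio to the character; EnableControl unlocks and toggles it.
; Tick drives a delay-throttled check that optionally flips the notifier toward the player's side.
; CloseDoor, called ten seconds after opening, is empty, so nothing auto-closes here.
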(event Custom|InfoNotifierLocation
  (bind _notifier_location (Variables|Default|GetNotifier_Location))
  (Utilities|FlowControl|Delay 0.2)
  (if (Variables|Default|GetbPositionBasedNotifier)
    (Variables|Default|SetPlayerLocation (.x (.location (Class|KismetMathLibrary|ConvertTransformtoRelative (Transformation|GetWorldTransform (Variables|Character|GetMesh)) (Transformation|GetActorTransform (Game|Player|GetPlayerPawn 0))))))
    (if (< (Variables|Default|GetPlayerLocation) 0.0)
      (Transformation|SetRelativeRotation _notifier_location "0,180.000000, 0" false false)
      (else
        (Transformation|SetRelativeRotation _notifier_location "0, 0, 0" false false)))))

(event Custom|OpenDoor
  (Utilities|FlowControl|FlipFlop
    (:A
      (bind _rotate (Timeline|DoorOpen Play)
        (:Update
          (Transformation|SetRelativeRotation (Variables|Character|GetMesh) (Math|Rotator|MakeRotator 0.0 0.0 (* _rotate (Variables|Default|GetDoorOpenAmount))) false false))
        (:Finished
          (Utilities|FlowControl|Delay 1e+01)
          (CallFunction|CloseDoor))))
    (:B
      (Timeline|DoorOpen Reverse))))

(event Custom|CloseDoor)

(event Custom|EnableControl
  (Variables|Default|SetDisableControl false)
  (CallFunction|OpenDoor))

(event EventBeginPlay
  (|CallParentFunction)
  (Transformation|AttachComponentToComponent (Variables|Default|GetNotifier_Location) (Variables|Character|GetMesh) "None" "KeepWorld" "KeepWorld" "KeepWorld" true)
  (if (Variables|Default|GetInitialOpen)
    (CallFunction|OpenDoor)))

(event Collision|EventActorBeginOverlap
  (params (OtherActor :type Actor%20Object%20Reference))
  (|CallParentFunction OtherActor) ; This node is disabled and will not be called.\nDrag off pins to build functionality.
)

(event EventTick
  (params (DeltaSeconds :type Float%20%28single-precision%29))
  (|CallParentFunction DeltaSeconds)
  (CallFunction|InfoNotifierLocation))

(fn ConstructionScript
  (|CallParentFunction))

(fn Interact
  (params (Actor :type Actor%20Object%20Reference))
  (if (Variables|Default|GetDisableControl)
    (bind _ascharacter_base_bp (Utilities|Casting|CastToCharacterBase_BP Actor)
      (:then
        (Default|UpdateTextandPlayAudio _ascharacter_base_bp 8 (Variables|Default|GetDoorText) false (Variables|Default|GetSoundAsset)))
      (:CastFailed
        (return 0 false)))
    (else
      (Variables|Default|SetCharacterLocation (Transformation|GetActorLocation Actor))
      (CallFunction|OpenDoor)
      (return 0 false))))