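; Remote_BP is an interactive actor Blueprint, named as a remote, that currently has no gameplay behavior of its own.
; It declares interaction functions for detection, range, info bubbles, keep-back and interact, all stubs that return false, with Interact reporting not attached.
; Its construction script only calls the parent, and its event graph holds only disabled placeholder events.
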(event EventBeginPlay
  (|CallParentFunction) ; This node is disabled and will not be called.\nDrag off pins to build functionality.
)

(event Collision|EventActorBeginOverlap
  (params (OtherActor :type Actor%20Object%20Reference)))

(event EventTick
  (params (DeltaSeconds :type Float%20%28single-precision%29))
  (|CallParentFunction DeltaSeconds) ; This node is disabled and will not be called.\nDrag off pins to build functionality.
)

(fn ConstructionScript
  (|CallParentFunction))

(fn InfoBubbleDown
  (return false))

(fn InfoBubbleUp
  (return false))

(fn OutOfRange
  (return false))

(fn KeepBack
  (params (CurrentLocation :type Vector :default "0, 0, 0") (CurrentRotation :type Rotator :default "0, 0, 0"))
  (return false))

(fn Interact
  (params (Actor :type Actor%20Object%20Reference))
  (return 0 false))

(fn Detected
  (return false))