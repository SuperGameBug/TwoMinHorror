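; Interactive TV actor that the player can switch on and off, with screen state shown by swapping a material on its Plane mesh.
; A box overlap by CharacterBase_BP adds or removes a HUD_UMG press-E prompt and sets PlayerInRange.
; Interact toggles TVState and the screen, while the other interaction functions are stubs returning false.
; BeginPlay runs a timed off-on-off sequence without changing TVState.
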(event OnComponentBeginOverlap(Box)
  (params (OverlappedComponent :type Primitive%20Component%20Object%20Reference) (OtherActor :type Actor%20Object%20Reference) (OtherComp :type Primitive%20Component%20Object%20Reference) (OtherBodyIndex :type Integer) (bFromSweep :type Boolean) (SweepResult :type Hit%20Result%20Structure%20%28by%20ref%29))
  (Utilities|Casting|CastToCharacterBase_BP OtherActor)
  (Utilities|IsValid (Variables|Default|GetPressEWidget)
    (:Is%20Valid
      _)
    (:Is%20Not%20Valid
      (bind _returnvalue (UserInterface|CreateWidget "/Game/Blueprints/UMG/UserInterFace/HUD_UMG.HUD_UMG_C"))))
  (bind _output_get (Variables|Default|SetPressEWidget _returnvalue))
  (UserInterface|Viewport|AddtoViewport _output_get 0)
  (Variables|Default|SetPlayerInRange true))

(event OnComponentEndOverlap(Box)
  (params (OverlappedComponent :type Primitive%20Component%20Object%20Reference) (OtherActor :type Actor%20Object%20Reference) (OtherComp :type Primitive%20Component%20Object%20Reference) (OtherBodyIndex :type Integer))
  (Utilities|Casting|CastToCharacterBase_BP OtherActor)
  (Widget|RemovefromParent (Variables|Default|GetPressEWidget))
  (Variables|Default|SetPlayerInRange false))

(event Custom|TV_OnOff
  (params (State :type Boolean))
  (if State
    (Rendering|Material|SetMaterial (Variables|Default|GetPlane) 1 "/Game/Assets/Materials/GenericMaterials/MI_LIght_2.MI_LIght_2")
    (else
      (Rendering|Material|SetMaterial (Variables|Default|GetPlane) 1 "/Game/Assets/Materials/GenericMaterials/MI_plastic_2.MI_plastic_2"))))

(event EventBeginPlay
  (CallFunction|TVonOff false)
  (Utilities|FlowControl|Delay 3.0)
  (CallFunction|TVonOff true)
  (Utilities|FlowControl|Delay 3.0)
  (CallFunction|TVonOff false))

(fn ConstructionScript)

(fn Detected
  (return false))

(fn InfoBubbleDown
  (return false))

(fn InfoBubbleUp
  (return false))

(fn Interact
  (params (Actor :type Actor%20Object%20Reference))
  (if (Variables|Default|GetTVState)
    (CallFunction|TVonOff false)
    (else
      (CallFunction|TVonOff true)))
  (Variables|Default|SetTVState (not (Variables|Default|GetTVState)))
  (return 0 false))

(fn KeepBack
  (params (CurrentLocation :type Vector :default "0, 0, 0") (CurrentRotation :type Rotator :default "0, 0, 0"))
  (return false))

(fn OutOfRange
  (return false))