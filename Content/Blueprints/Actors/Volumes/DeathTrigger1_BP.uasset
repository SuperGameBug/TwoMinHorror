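; DeathTrigger1_BP is a one-shot story trigger volume that stages the Nikki death scene when the character overlaps its box while ActivateTrigger is set.
; It slows the player, opens the tagged Nikki room door, reveals the NikkiDead mesh, raises MomCry volume and arms FinalTrigger_BP.
; It then disables every door, with a delay inside that loop leading to the player's voiced, subtitled reaction.
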(event OnComponentBeginOverlap(Box)
  (params (OverlappedComponent :type Primitive%20Component%20Object%20Reference) (OtherActor :type Actor%20Object%20Reference) (OtherComp :type Primitive%20Component%20Object%20Reference) (OtherBodyIndex :type Integer) (bFromSweep :type Boolean) (SweepResult :type Hit%20Result%20Structure%20%28by%20ref%29))
  (bind _ascharacter_base_bp (Utilities|Casting|CastToCharacterBase_BP OtherActor))
  (if (Variables|Default|GetActivateTrigger)
    (Utilities|FlowControl|DoOnce false
      (:Completed
        (Variables|/Script/Engine.CharacterMovementComponent|SetMaxWalkSpeed (Variables|/Script/Engine.Character|GetCharacterMovement _ascharacter_base_bp) 1e+02)
        (bind _outactors (Actor|GetAllActorswithTag "nikkiroomdoor"))
        (bind _asdoor_bp (Utilities|Casting|CastToDoor_BP (Utilities|Array|Get(acopy) _outactors)))
        (Default|OpenDoor _asdoor_bp)
        (Variables|/Game/Blueprints/Actors/Interactive/Door_BP.Door_BP_C|SetDisableControl _asdoor_bp false)
        (bind _outactors_2 (Actor|GetAllActorsOfClass "/Game/Blueprints/Actors/NPC/NikkiDead_BP.NikkiDead_BP_C"))
        (Rendering|SetVisibility (Variables|/Game/Blueprints/Actors/NPC/NikkiDead_BP.NikkiDead_BP_C|GetSM_Nikki_01_Dead (Utilities|Array|Get(acopy) _outactors_2)) true true)
        (Audio|Components|Audio|SetVolumeMultiplier (Variables|/Game/Blueprints/Actors/NPC/NikkiDead_BP.NikkiDead_BP_C|GetMomCry (Utilities|Array|Get(acopy) _outactors_2)) 1.0 :!class /Script/Engine.AudioComponent)
        (bind _outactors_3 (Actor|GetAllActorsOfClass "/Game/Blueprints/Actors/Helpers/FinalTrigger_BP.FinalTrigger_BP_C"))
        (Variables|/Game/Blueprints/Actors/Helpers/FinalTrigger_BP.FinalTrigger_BP_C|SetTriggerEnabled (Utilities|Array|Get(acopy) _outactors_3) true)
        (bind _outactors_4 (Actor|GetAllActorsOfClass "/Game/Blueprints/Actors/Interactive/Door_BP.Door_BP_C"))
        (for _array_element _outactors_4
          (Variables|/Game/Blueprints/Actors/Interactive/Door_BP.Door_BP_C|SetDisableEverything _array_element true)
          (Utilities|FlowControl|Delay 6.0)
          (Default|UpdateTextandPlayAudio _ascharacter_base_bp 0 "Is that... mom…? What’s going on in the house !?" false "/Game/Assets/Audio/VoiceOvers/Nikki/21-_Is_that_mom.21-_Is_that_mom"))))))

(event EventBeginPlay)

(event Collision|EventActorBeginOverlap
  (params (OtherActor :type Actor%20Object%20Reference)))

(event EventTick
  (params (DeltaSeconds :type Float%20%28single-precision%29)))

(fn ConstructionScript)