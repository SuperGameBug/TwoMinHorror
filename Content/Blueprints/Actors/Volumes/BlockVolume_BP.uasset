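; BlockVolume_BP is a volume actor that slows characters near a gated area until Level 2 is unlocked.
; On BeginPlay it finds the first ProgressTracker_BP and binds its UnlockLevel2 event to destroy this actor.
; PhysBound overlaps cut a CharacterBase_BP's walk speed when its Pawn-type component enters, then set a hardcoded normal speed on exit rather than restoring the previous value.
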(event OnComponentBeginOverlap(PhysBound)
  (params (OverlappedComponent :type Primitive%20Component%20Object%20Reference) (OtherActor :type Actor%20Object%20Reference) (OtherComp :type Primitive%20Component%20Object%20Reference) (OtherBodyIndex :type Integer) (bFromSweep :type Boolean) (SweepResult :type Hit%20Result%20Structure%20%28by%20ref%29))
  (bind _ascharacter_base_bp (Utilities|Casting|CastToCharacterBase_BP OtherActor))
  (if (Utilities|Enum|Equal(Enum) (Collision|GetCollisionObjectType OtherComp) "ECC_Pawn")
    (Variables|/Script/Engine.CharacterMovementComponent|SetMaxWalkSpeed (Variables|/Script/Engine.Character|GetCharacterMovement _ascharacter_base_bp) 5e+01)))

(event OnComponentEndOverlap(PhysBound)
  (params (OverlappedComponent :type Primitive%20Component%20Object%20Reference) (OtherActor :type Actor%20Object%20Reference) (OtherComp :type Primitive%20Component%20Object%20Reference) (OtherBodyIndex :type Integer))
  (bind _ascharacter_base_bp (Utilities|Casting|CastToCharacterBase_BP OtherActor))
  (if (Utilities|Enum|Equal(Enum) (Collision|GetCollisionObjectType OtherComp) "ECC_Pawn")
    (Variables|/Script/Engine.CharacterMovementComponent|SetMaxWalkSpeed (Variables|/Script/Engine.Character|GetCharacterMovement _ascharacter_base_bp) 1.5e+02)))

(event Custom|Destroy
  (Actor|DestroyActor))

(event EventBeginPlay
  (bind _outactors (Actor|GetAllActorsOfClass "/Game/Blueprints/Actors/Helpers/ProgressTracker_BP.ProgressTracker_BP_C"))
  (bind _asprogress_tracker_bp (Utilities|Casting|CastToProgressTracker_BP (Utilities|Array|Get(acopy) _outactors)))
  (EventDispatchers|BindEventtoUnlockLevel2 _asprogress_tracker_bp (delegate Custom|Destroy)))

(event Collision|EventActorBeginOverlap
  (params (OtherActor :type Actor%20Object%20Reference)))

(event EventTick
  (params (DeltaSeconds :type Float%20%28single-precision%29)))

(fn ConstructionScript)