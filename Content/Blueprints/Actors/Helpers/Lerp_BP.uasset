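; Trigger-box helper actor that moves the player character through a scripted location lerp when entered.
; When enabled, an overlap by a CharacterBase_BP component tagged BaseCapsule fires once and passes this instance's Lerpindex to the character's LerpActorLocation.
; One specific index also plays a two-part inner monologue through the character's text-and-audio function, separated by a short delay.
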(event OnComponentBeginOverlap(PlayerDetectionBox)
  (params (OverlappedComponent :type Primitive%20Component%20Object%20Reference) (OtherActor :type Actor%20Object%20Reference) (OtherComp :type Primitive%20Component%20Object%20Reference) (OtherBodyIndex :type Integer) (bFromSweep :type Boolean) (SweepResult :type Hit%20Result%20Structure%20%28by%20ref%29))
  (bind _lerpindex (Variables|Default|Getlerpindex))
  (bind _ascharacter_base_bp (Utilities|Casting|CastToCharacterBase_BP OtherActor))
  (if (and (Variables|Default|GetTriggerEnabled) (Components|ComponentHasTag OtherComp "BaseCapsule"))
    (Utilities|FlowControl|DoOnce false
      (:Completed
        (Default|LerpActorLocation _ascharacter_base_bp _lerpindex)
        (if (== _lerpindex 4)
          (Default|UpdateTextandPlayAudio _ascharacter_base_bp 0 "It’s been so long since I have felt the solace. 
No bullies, no teachers who don’t give a damn, no judgmental family and friends," false "/Game/Assets/Audio/TestVoiceOvers/2.2")
          (Utilities|FlowControl|Delay 3.0)
          (Default|UpdateTextandPlayAudio _ascharacter_base_bp 0 "not feeling like I'm a loser…  
but then again, I shouldn’t get used to feeling good only when I’m talking to myself,right? 
" false "/Game/Assets/Audio/TestVoiceOvers/2.2"))))))

(event EventBeginPlay)

(event Collision|EventActorBeginOverlap
  (params (OtherActor :type Actor%20Object%20Reference)))

(event EventTick
  (params (DeltaSeconds :type Float%20%28single-precision%29)))

(fn ConstructionScript)