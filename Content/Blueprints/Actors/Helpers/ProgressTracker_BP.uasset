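; ProgressTracker_BP is a helper actor that counts completed objectives and signals when levels 2 and 3 unlock.
; IncrementObjective inserts the incremented count at the given ObjectiveCompleted index, shifting older entries along rather than overwriting them.
; It fires the UnlockLevel2 dispatcher when the first count equals its NumberOfObjective target.
; Only within that branch does it compare the second count and fire UnlockLevel3.
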(event Custom|IncrementObjective
  (params (NewParam :type Integer))
  (Utilities|Array|Insert (Variables|Default|GetObjectiveCompleted) (+ (Utilities|Array|Get(acopy) (Variables|Default|GetObjectiveCompleted) NewParam) 1) NewParam)
  (if (== (Utilities|Array|Get(acopy) (Variables|Default|GetObjectiveCompleted)) (Utilities|Array|Get(acopy) (Variables|Default|GetNumberOfObjective)))
    (Default|CallUnlockLevel2)
    (if (== (Utilities|Array|Get(acopy) (Variables|Default|GetObjectiveCompleted) 1) (Utilities|Array|Get(acopy) (Variables|Default|GetNumberOfObjective) 1))
      (Default|CallUnlockLevel3))))

(event EventBeginPlay)

(event Collision|EventActorBeginOverlap
  (params (OtherActor :type Actor%20Object%20Reference)))

(event EventTick
  (params (DeltaSeconds :type Float%20%28single-precision%29)))

(fn ConstructionScript)