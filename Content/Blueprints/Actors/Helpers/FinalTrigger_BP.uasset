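; Final story trigger actor that plays an ending beat when the player character's base capsule enters its detection box.
; While enabled, the overlap fires once, calls LerpActorLocation on the character, then after a delay shows a closing subtitle with voice audio.
; Longer dialogue, end-credits widget and end level sequence logic remain in the graph but are disconnected, so nothing follows the last delay.
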(event OnComponentBeginOverlap(PlayerDetectionBox)
  (params (OverlappedComponent :type Primitive%20Component%20Object%20Reference) (OtherActor :type Actor%20Object%20Reference) (OtherComp :type Primitive%20Component%20Object%20Reference) (OtherBodyIndex :type Integer) (bFromSweep :type Boolean) (SweepResult :type Hit%20Result%20Structure%20%28by%20ref%29))
  (bind _ascharacter_base_bp (Utilities|Casting|CastToCharacterBase_BP OtherActor))
  (if (and (Variables|Default|GetTriggerEnabled) (Components|ComponentHasTag OtherComp "BaseCapsule"))
    (Utilities|FlowControl|DoOnce false
      (:Completed
        (Default|LerpActorLocation _ascharacter_base_bp 5)
        (Utilities|FlowControl|Delay 3.0)
        (Default|UpdateTextandPlayAudio _ascharacter_base_bp 0 "Oh yeah...I guess I really couldn’t take it tonight." false "/Game/Assets/Audio/VoiceOvers/Nikki/22-_Oh_yeah_I_guess_I_really_couldn_t_take_it_tonight.22-_Oh_yeah_I_guess_I_really_couldn_t_take_it_tonight")
        (Utilities|FlowControl|Delay 5.0)))))

(event EventBeginPlay)

(event Collision|EventActorBeginOverlap
  (params (OtherActor :type Actor%20Object%20Reference)))

(event EventTick
  (params (DeltaSeconds :type Float%20%28single-precision%29)))

(fn ConstructionScript)