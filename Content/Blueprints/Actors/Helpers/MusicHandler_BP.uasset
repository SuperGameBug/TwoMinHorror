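; MusicHandler_BP is a helper Blueprint that controls main menu and gameplay background music.
; SwitchMusic fades the menu track in or out with an S-curve based on a MainMenu flag; the gameplay track's fade nodes are disconnected, so it is never switched here.
; ChangeMusicVol applies one volume multiplier to both tracks and returns true.
; The event graph has no active logic.
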(event EventBeginPlay)

(event Collision|EventActorBeginOverlap
  (params (OtherActor :type Actor%20Object%20Reference)))

(event EventTick
  (params (DeltaSeconds :type Float%20%28single-precision%29)))

(fn ConstructionScript)

(fn SwitchMusic
  (params (mainMenu :type Boolean))
  (if mainMenu
    (Audio|Components|Audio|FadeIn (Variables|Default|GetMainMenuMusic) 5.0 1.0 0.0 "SCurve" :!class /Script/Engine.AudioComponent)
    (else
      (Audio|Components|Audio|FadeOut (Variables|Default|GetMainMenuMusic) 5.0 0.0 "SCurve" :!class /Script/Engine.AudioComponent))))

(fn ChangeMusicVol
  (params (Volume :type Float%20%28single-precision%29))
  (Audio|Components|Audio|SetVolumeMultiplier (Variables|Default|GetMainMenuMusic) Volume :!class /Script/Engine.AudioComponent)
  (Audio|Components|Audio|SetVolumeMultiplier (Variables|Default|GetGameBackgroundMusic) Volume :!class /Script/Engine.AudioComponent)
  (return true))