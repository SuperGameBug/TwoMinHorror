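; Helper trigger volume that swaps a character's walking sound while it is inside the box, for use on staircases.
; Box overlap begin sets the CharacterBase_BP Walk audio component to the staircase climb sound, and overlap end restores the player walking sound.
; Only overlaps from components tagged BaseCapsule count, so other parts of the character do not trigger the swap.
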(event OnComponentBeginOverlap(Box)
  (params (OverlappedComponent :type Primitive%20Component%20Object%20Reference) (OtherActor :type Actor%20Object%20Reference) (OtherComp :type Primitive%20Component%20Object%20Reference) (OtherBodyIndex :type Integer) (bFromSweep :type Boolean) (SweepResult :type Hit%20Result%20Structure%20%28by%20ref%29))
  (bind _ascharacter_base_bp (Utilities|Casting|CastToCharacterBase_BP OtherActor))
  (if (Components|ComponentHasTag OtherComp "BaseCapsule")
    (Audio|Components|Audio|SetSound (Variables|/Game/Blueprints/Pawns/CharacterBase_BP.CharacterBase_BP_C|GetWalk _ascharacter_base_bp) "/Game/Assets/Audio/SFX/SFX_StaircaseClimb.SFX_StaircaseClimb")))

(event OnComponentEndOverlap(Box)
  (params (OverlappedComponent :type Primitive%20Component%20Object%20Reference) (OtherActor :type Actor%20Object%20Reference) (OtherComp :type Primitive%20Component%20Object%20Reference) (OtherBodyIndex :type Integer))
  (bind _ascharacter_base_bp (Utilities|Casting|CastToCharacterBase_BP OtherActor))
  (if (Components|ComponentHasTag OtherComp "BaseCapsule")
    (Audio|Components|Audio|SetSound (Variables|/Game/Blueprints/Pawns/CharacterBase_BP.CharacterBase_BP_C|GetWalk _ascharacter_base_bp) "/Game/Assets/Audio/SFX/SFX_PlayerWalking.SFX_PlayerWalking")))

(event EventBeginPlay)

(event Collision|EventActorBeginOverlap
  (params (OtherActor :type Actor%20Object%20Reference)))

(event EventTick
  (params (DeltaSeconds :type Float%20%28single-precision%29)))

(fn ConstructionScript)