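; Wall horror decal actor that keeps three decals hidden until they are revealed.
; BeginPlay creates dynamic material instances for the decals and sets their Opacity parameter to zero.
; The DecalAppears event creates the instances again and plays a timeline that drives all three opacities together.
; Nothing in this graph triggers DecalAppears, as its only call here is unconnected.
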(event Custom|DecalAppears
  (bind _returnvalue (Rendering|Material|CreateDynamicMaterialInstance (Variables|Default|GetDecal) :!class /Script/Engine.DecalComponent))
  (bind _returnvalue_2 (Rendering|Material|CreateDynamicMaterialInstance (Variables|Default|GetDecal2) :!class /Script/Engine.DecalComponent))
  (bind _returnvalue_3 (Rendering|Material|CreateDynamicMaterialInstance (Variables|Default|GetDecal1) :!class /Script/Engine.DecalComponent))
  (bind _newtrack_0 (Timeline|Timeline_0 PlayFromStart)
    (:Update
      (Rendering|Material|SetScalarParameterValue _returnvalue "Opacity" _newtrack_0 :!class /Script/Engine.MaterialInstanceDynamic)
      (Rendering|Material|SetScalarParameterValue _returnvalue_2 "Opacity" _newtrack_0 :!class /Script/Engine.MaterialInstanceDynamic)
      (Rendering|Material|SetScalarParameterValue _returnvalue_3 "Opacity" _newtrack_0 :!class /Script/Engine.MaterialInstanceDynamic))))

(event EventBeginPlay
  (bind _returnvalue (Rendering|Material|CreateDynamicMaterialInstance (Variables|Default|GetDecal) :!class /Script/Engine.DecalComponent))
  (bind _returnvalue_2 (Rendering|Material|CreateDynamicMaterialInstance (Variables|Default|GetDecal2) :!class /Script/Engine.DecalComponent))
  (bind _returnvalue_3 (Rendering|Material|CreateDynamicMaterialInstance (Variables|Default|GetDecal1) :!class /Script/Engine.DecalComponent))
  (Rendering|Material|SetScalarParameterValue _returnvalue "Opacity" 0.0 :!class /Script/Engine.MaterialInstanceDynamic)
  (Rendering|Material|SetScalarParameterValue _returnvalue_2 "Opacity" 0.0 :!class /Script/Engine.MaterialInstanceDynamic)
  (Rendering|Material|SetScalarParameterValue _returnvalue_3 "Opacity" 0.0 :!class /Script/Engine.MaterialInstanceDynamic))

(fn ConstructionScript)