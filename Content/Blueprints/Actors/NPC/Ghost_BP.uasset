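; Ghost NPC scare actor that stays hidden until a character enters its trigger box while ActivateTrigger is set.
; It fires once, playing a player voice line with text and a scare sound while briefly showing the skeletal mesh.
; The instance tagged "ghost2" also slows the character, opens the "topdoor" door and disables its input, and arms the first DeathTrigger1_BP to continue the sequence.
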(event OnComponentBeginOverlap(Box)
  (params (OverlappedComponent :type Primitive%20Component%20Object%20Reference) (OtherActor :type Actor%20Object%20Reference) (OtherComp :type Primitive%20Component%20Object%20Reference) (OtherBodyIndex :type Integer) (bFromSweep :type Boolean) (SweepResult :type Hit%20Result%20Structure%20%28by%20ref%29))
  (bind _ascharacter_base_bp (Utilities|Casting|CastToCharacterBase_BP OtherActor))
  (if (Variables|Default|GetActivateTrigger)
    (Utilities|FlowControl|DoOnce false
      (:Completed
        (CallFunction|GhostAppear _ascharacter_base_bp)
        (if (Actor|ActorHasTag "ghost2")
          (Variables|/Script/Engine.CharacterMovementComponent|SetMaxWalkSpeed (Variables|/Script/Engine.Character|GetCharacterMovement _ascharacter_base_bp) 5e+01)
          (bind _outactors (Actor|GetAllActorswithTag "topdoor"))
          (bind _asdoor_bp (Utilities|Casting|CastToDoor_BP (Utilities|Array|Get(acopy) _outactors)))
          (Input|DisableInput _asdoor_bp 0)
          (Default|OpenDoor _asdoor_bp)
          (bind _outactors_2 (Actor|GetAllActorsOfClass "/Game/Blueprints/Actors/Volumes/DeathTrigger1_BP.DeathTrigger1_BP_C"))
          (Variables|/Game/Blueprints/Actors/Volumes/DeathTrigger1_BP.DeathTrigger1_BP_C|SetActivateTrigger (Utilities|Array|Get(acopy) _outactors_2) true))))))

(event Custom|GhostAppear
  (params (CharacterRef :type Character%20Base%20BP%20Object%20Reference))
  (Default|UpdateTextandPlayAudio CharacterRef 0 " what?! Fuck it, I’m outta here!" false "/Game/Assets/Audio/VoiceOvers/Nikki/20-_Fuck_it__I_m_out_of_here.20-_Fuck_it__I_m_out_of_here")
  (Audio|PlaySound2D (Variables|Default|GetScarySound) 1.0 1.0 0.0 0 0)
  (Rendering|SetVisibility (Variables|Default|GetSkeletalMesh) true true)
  (Utilities|FlowControl|Delay 2.0)
  (Rendering|SetVisibility (Variables|Default|GetSkeletalMesh) false true))

(event EventBeginPlay
  (Rendering|SetVisibility (Variables|Default|GetSkeletalMesh) false true))

(fn ConstructionScript)